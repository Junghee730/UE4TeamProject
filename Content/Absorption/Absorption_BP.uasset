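; Absorption pickup actor that passes its HP value to the player game instance subsystem, noted as an HP gain from enemy death.
; A one-second delay after BeginPlay arms it and prints the player's location.
; Once armed, any other actor overlapping AbsBox triggers SetAddDamage with AbsorptionHp and destroys it.
; On destruction, it adds a PlayerCube child actor component to the player, using player world location plus an offset as relative location.
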(event OnComponentBeginOverlap(absBox)
  (params (OverlappedComponent :type Primitive%20Component%20Object%20Reference) (OtherActor :type Actor%20Object%20Reference) (OtherComp :type Primitive%20Component%20Object%20Reference) (OtherBodyIndex :type Integer) (bFromSweep :type Boolean) (SweepResult :type Hit%20Result%20Structure%20%28by%20ref%29))
  ;[1 1 1] Absorption Enemy Die => PlayerAddHp
  (if (Variables|Default|GetAbsorptionSpawnCheck)
    (if (!= OtherActor self)
      (Class|PlayerGameInstanceSubsystem|SetAddDamage (Subsystems|GetPlayerGameInstanceSubsystem) (Variables|Default|GetAbsorptionHp))
      (Actor|DestroyActor))))

(event EventBeginPlay
  ;[1 1 1] Absorption Spawn Check
  (Utilities|FlowControl|Delay 1.0)
  (Variables|Default|SetAbsorptionSpawnCheck true)
  (bind _asthird_person_character (Utilities|Casting|CastToThirdPersonCharacter (Game|GetPlayerCharacter 0)))
  (Development|PrintString (Utilities|String|ToString(Vector) (Transformation|GetActorLocation _asthird_person_character)) true true "(R=0.000000,G=0.660000,B=1.000000,A=1.000000)" 8e+01))

(event EventTick
  (params (DeltaSeconds :type Float%20%28single-precision%29)))

(event EventDestroyed
  (bind _asthird_person_character (Utilities|Casting|CastToThirdPersonCharacter (Game|GetPlayerCharacter 0)))
  (bind _returnvalue (AddComponent|AddChildActorComponent _asthird_person_character (Class|Actor|IsChildActor _asthird_person_character) (Math|Conversions|ToTransform(Vector) (Transformation|GetActorLocation _asthird_person_character))))
  (ChildActorComponent|SetChildActorClass _returnvalue "/Game/Absorption/PlayerCube.PlayerCube_C")
  (Transformation|SetRelativeTransform _returnvalue (Math|Transform|MakeTransform (+ (Transformation|GetActorLocation _asthird_person_character) "700.000000,-400.000000,-300.000000") "0, 0, 0" "1,1,1") false false))

(fn ConstructionScript)